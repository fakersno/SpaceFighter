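; LargeBall is a wandering actor in the Advanced Lockon System, tagged with its team and type.
; On BeginPlay it sets those tags, applies its material and stores its spawn location as the origin.
; Each tick it interpolates toward a random point in a box around that origin, without sweeping, and picks a new point on arrival.
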(event `self.ReceiveBeginPlay`
  (set `self.Tags` (`|MakeArray` (`self.Team`) (`KismetStringLibrary.Conv_StringToName` (`|GetEnumeratorNameAsString` (`self.Type`)))))
  (`PrimitiveComponent.SetMaterial` (`self.StaticMesh`) 0 (`self.Material`))
  (set `self.Origin` (`self.K2_GetActorLocation`))
  (`self.Set Target`))

(event `Set Target`
  (set `self.Target` (`KismetMathLibrary.RandomPointInBoundingBox` (`self.Origin`) (`KismetMathLibrary.MakeVector` 2500.0 1000.0 1500.0)))
  (set `self.Moving` true))

(event `self.ReceiveTick`
  (params (DeltaSeconds :type "Float (single-precision)"))
  (set `self.DeltaTime` DeltaSeconds)
  (if (`self.Moving`)
    (`self.K2_SetActorLocation` (`KismetMathLibrary.VInterpTo` (`self.K2_GetActorLocation`) (`self.Target`) (`self.DeltaTime`) 3.0))
    (if (== (`self.K2_GetActorLocation`) (`self.Target`) :`ErrorTolerance` 1.0)
      (set `self.Moving` false)
      (`self.Set Target`))))

(fn `UserConstructionScript`)