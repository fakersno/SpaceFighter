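; Ball is a moving actor in the lock-on system that tags itself with its team and type and applies its material on begin play.
; Each tick, Mode selects the movement, eased with VInterpTo.
; One mode wanders between random points in a box around the start location; the other shuttles between the start and a fixed offset along world X.
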(event `self.ReceiveBeginPlay`
  (set `self.Tags` (`|MakeArray` (`self.Team`) (`KismetStringLibrary.Conv_StringToName` (`|GetEnumeratorNameAsString` (`self.Type`)))))
  (`PrimitiveComponent.SetMaterial` (`self.StaticMesh`) 0 (`self.Material`))
  (set `self.Origin` (`self.K2_GetActorLocation`))
  (`self.Set Target`)
  (set `self.Target2` (+ (`self.Origin`) (400.0 0.0 0.0))))

(event `Set Target`
  (set `self.Target` (`KismetMathLibrary.RandomPointInBoundingBox` (`self.Origin`) (`KismetMathLibrary.MakeVector` 250.0 100.0 150.0)))
  (set `self.Moving` true))

(event `self.ReceiveTick`
  (params (DeltaSeconds :type "Float (single-precision)"))
  (set `self.DeltaTime` DeltaSeconds)
  (switch `int` (`self.Mode`)
    (:`1`
      (if (`self.Moving`)
        (`self.K2_SetActorLocation` (`KismetMathLibrary.VInterpTo` (`self.K2_GetActorLocation`) (`self.Target`) (`self.DeltaTime`) 3.0))
        (if (== (`self.K2_GetActorLocation`) (`self.Target`) :`ErrorTolerance` 1.0)
          (set `self.Moving` false)
          (`self.Set Target`))))
    (:`2`
      (if (`self.Forwad`)
        (`self.K2_SetActorLocation` (`KismetMathLibrary.VInterpTo` (`self.K2_GetActorLocation`) (`self.Target2`) (`self.DeltaTime`) 1.0))
        (if (== (`self.K2_GetActorLocation`) (`self.Target2`) :`ErrorTolerance` 1.0)
          (set `self.Forwad` false))
        (else
          (`self.K2_SetActorLocation` (`KismetMathLibrary.VInterpTo` (`self.K2_GetActorLocation`) (`self.Origin`) (`self.DeltaTime`) 1.0))
          (if (== (`self.K2_GetActorLocation`) (`self.Origin`) :`ErrorTolerance` 1.0)
            (set `self.Forwad` true)))))))

(fn `UserConstructionScript`)