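; TestShip is a test ship actor for the Advanced Lockon System that launches homing SAM missiles at a target.
; On BeginPlay it tags itself with a team and type, applies its material and, if enabled, starts a looping timer.
; Each tick of that timer spawns a launch effect and a SAM oriented by a mesh socket, then homes it on Target.
; A delayed for-loop macro is defined but not called.
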(event `self.ReceiveBeginPlay`
  (set `self.Tags` (`|MakeArray` (`self.Team`) (`KismetStringLibrary.Conv_StringToName` (`|GetEnumeratorNameAsString` (`self.Type`)))))
  (`PrimitiveComponent.SetMaterial` (`self.StaticMesh`) 0 (`self.Material`))
  (if (`self.Enable`)
    (`KismetSystemLibrary.K2_SetTimerDelegate` (delegate `SingleFire`) 2.0 true)))

(event `SingleFire`
  (bind _returnvalue (`SceneComponent.K2_GetComponentLocation` (`self.StaticMesh`)))
  (`GameplayStatics.SpawnEmitterAtLocation` "/Game/AdvancedLockonSystem/EpicDemoContent/Effects/ParticleSystems/Weapons/RocketLauncher/Impact/P_Launcher_IH.P_Launcher_IH" _returnvalue)
  (bind _returnvalue_2 (`|SpawnActorFromClass` "/Game/AdvancedLockonSystem/Blueprints/Actor/Projectile/SAM.SAM_C" (`KismetMathLibrary.MakeTransform` _returnvalue (`SceneComponent.GetSocketRotation` (`self.StaticMesh`) "1")) "AdjustIfPossibleButAlwaysSpawn" "OverrideRootScale" self null))
  (`/Game/AdvancedLockonSystem/Blueprints/Actor/Projectile/SAM.Homing` _returnvalue_2 (`self.Target`)))

(fn `UserConstructionScript`)