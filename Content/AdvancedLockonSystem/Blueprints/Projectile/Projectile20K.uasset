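; Projectile actor in the Advanced Lockon System that damages whatever it hits and explodes.
; On BeginPlay it replaces its actor tags with its owner's first tag and the name of its Type enum value.
; On Hit it applies fixed damage to the struck actor, spawns a half-scale launcher impact effect with an explosion sound, then destroys itself.
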(event `self.ReceiveBeginPlay`
  ;[1 1 1] Set actor tags
  (set `self.Tags` (`|MakeArray` (`|GetArrayItem` (`Actor.Tags` (`self.GetOwner`))) (`KismetStringLibrary.Conv_StringToName` (`|GetEnumeratorNameAsString` (`self.Type`))))))

(event `self.ReceiveHit`
  (params (MyComp :type "PrimitiveComponent Object Reference") (Other :type "Actor Object Reference") (OtherComp :type "PrimitiveComponent Object Reference") (bSelfMoved :type Boolean) (HitLocation :type "Vector Structure") (HitNormal :type "Vector Structure") (NormalImpulse :type "Vector Structure") (Hit :type "HitResult Structure (by ref)"))
  (`GameplayStatics.ApplyDamage` Other 100.0)
  (`GameplayStatics.SpawnEmitterAtLocation` "/Game/AdvancedLockonSystem/EpicDemoContent/Effects/ParticleSystems/Weapons/RocketLauncher/Impact/P_Launcher_IH.P_Launcher_IH" HitLocation (struct) (0.5 0.5 0.5))
  (`GameplayStatics.PlaySoundAtLocation` "/Game/AdvancedLockonSystem/EpicDemoContent/Sounds/Cue/GrenadeLauncher_Explosion_Cue.GrenadeLauncher_Explosion_Cue" HitLocation)
  (`self.K2_DestroyActor`))

(fn `UserConstructionScript`)