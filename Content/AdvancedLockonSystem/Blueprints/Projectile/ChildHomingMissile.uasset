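; Homing missile projectile in the lock-on system that explodes on impact, dealing damage to what it hits.
; On spawn it tags itself with its owner's first tag and its type; the Homing event points ProjectileMovement at the supplied target's root component.
; A looping timer checks the target and, if it is invalid, detonates the missile after a short delay.
; Any damage to the missile also detonates it, so it can be shot down.
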(event `self.ReceiveBeginPlay`
  ;[1 1 1] Set actor tags
  (set `self.Tags` (`|MakeArray` (`|GetArrayItem` (`Actor.Tags` (`self.GetOwner`))) (`KismetStringLibrary.Conv_StringToName` (`|GetEnumeratorNameAsString` (`self.Type`)))))
  (`KismetSystemLibrary.K2_SetTimerDelegate` (delegate `TargetCheck`) 1.0 true))

(event `TargetCheck`
  (bind _returnvalue (`self.K2_GetActorLocation`))
  ;[1 1 1] If the target is not valid, destroy self.
  (if (not (`KismetSystemLibrary.IsValid` (stale `Homing` HomingTarget)))
    (`KismetSystemLibrary.Delay` 3.0)
    (`GameplayStatics.SpawnEmitterAtLocation` "/Game/AdvancedLockonSystem/EpicDemoContent/Effects/ParticleSystems/Weapons/RocketLauncher/Impact/P_Launcher_IH.P_Launcher_IH" _returnvalue (struct) (5.0 5.0 5.0))
    (`GameplayStatics.PlaySoundAtLocation` "/Game/AdvancedLockonSystem/EpicDemoContent/Sounds/Cue/GrenadeLauncher_Explosion_Cue.GrenadeLauncher_Explosion_Cue" _returnvalue)
    (`self.K2_DestroyActor`)))

(event `Homing`
  (params (HomingTarget :type "Actor Object Reference"))
  (bind _projectilemovement (`self.ProjectileMovement`))
  ;[1 1 1] Set homing
  (if (`KismetSystemLibrary.IsValid` HomingTarget)
    (set `ProjectileMovementComponent.bIsHomingProjectile` true _projectilemovement)
    (set `ProjectileMovementComponent.HomingAccelerationMagnitude` 100000.0 _projectilemovement)
    (set `ProjectileMovementComponent.HomingTargetComponent` (`Actor.RootComponent` HomingTarget) _projectilemovement)))

(event `self.ReceiveHit`
  (params (MyComp :type "PrimitiveComponent Object Reference") (Other :type "Actor Object Reference") (OtherComp :type "PrimitiveComponent Object Reference") (bSelfMoved :type Boolean) (HitLocation :type "Vector Structure") (HitNormal :type "Vector Structure") (NormalImpulse :type "Vector Structure") (Hit :type "HitResult Structure (by ref)"))
  (`GameplayStatics.ApplyDamage` Other 100.0)
  (`GameplayStatics.SpawnEmitterAtLocation` "/Game/AdvancedLockonSystem/EpicDemoContent/Effects/ParticleSystems/Weapons/RocketLauncher/Impact/P_Launcher_IH.P_Launcher_IH" HitLocation (struct) (5.0 5.0 5.0))
  (`GameplayStatics.PlaySoundAtLocation` "/Game/AdvancedLockonSystem/EpicDemoContent/Sounds/Cue/GrenadeLauncher_Explosion_Cue.GrenadeLauncher_Explosion_Cue" HitLocation)
  (`self.K2_DestroyActor`))

(event `self.ReceiveAnyDamage`
  (params (Damage :type "Float (single-precision)") (DamageType :type "DamageType Object Reference") (InstigatedBy :type "Controller Object Reference") (DamageCauser :type "Actor Object Reference"))
  (bind _returnvalue (`self.K2_GetActorLocation`))
  (`GameplayStatics.SpawnEmitterAtLocation` "/Game/AdvancedLockonSystem/EpicDemoContent/Effects/ParticleSystems/Weapons/RocketLauncher/Impact/P_Launcher_IH.P_Launcher_IH" _returnvalue (struct) (5.0 5.0 5.0))
  (`GameplayStatics.PlaySoundAtLocation` "/Game/AdvancedLockonSystem/EpicDemoContent/Sounds/Cue/GrenadeLauncher_Explosion_Cue.GrenadeLauncher_Explosion_Cue" _returnvalue)
  (`self.K2_DestroyActor`))

(fn `UserConstructionScript`)