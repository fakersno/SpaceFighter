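; Supercarrier spaceship actor made of a carrier static mesh and four fighter meshes, with a selectable color scheme.
; The construction script switches on the Color variable and applies matching carrier and fighter material instances to slot 0 of each mesh.
; An unmatched value falls back to the black scheme.
; The event graph holds only disabled default events, so the actor has no runtime logic.
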(fn `UserConstructionScript`
  (bind _sm_gb4_supercarrier (`self.SM_GB4_SuperCarrier`))
  (bind _sm_gb4_supercarrier_fighter (`self.SM_GB4_Supercarrier_Fighter`))
  (bind _sm_gb4_supercarrier_fighter_1 (`self.SM_GB4_Supercarrier_Fighter_1`))
  (bind _sm_gb4_supercarrier_fighter_2 (`self.SM_GB4_Supercarrier_Fighter_2`))
  (bind _sm_gb4_supercarrier_fighter_3 (`self.SM_GB4_Supercarrier_Fighter_3`))
  (`|ExecutionSequence`
    (:`then_0`
      (switch `int` (`self.Color`)
        (:`Default`
          (`PrimitiveComponent.SetMaterial` _sm_gb4_supercarrier 0 "/Game/SpaceShips_Vol1/Materials/GB4_Supercarrier/MI_GB4_SuperCarrier_Black.MI_GB4_SuperCarrier_Black" :!label _label)
          (`PrimitiveComponent.SetMaterial` _sm_gb4_supercarrier_fighter 0 "/Game/SpaceShips_Vol1/Materials/GB4_Supercarrier/Fighter/MI_GB4_Fighter_Black.MI_GB4_Fighter_Black")
          (`PrimitiveComponent.SetMaterial` _sm_gb4_supercarrier_fighter_1 0 "/Game/SpaceShips_Vol1/Materials/GB4_Supercarrier/Fighter/MI_GB4_Fighter_Black.MI_GB4_Fighter_Black")
          (`PrimitiveComponent.SetMaterial` _sm_gb4_supercarrier_fighter_2 0 "/Game/SpaceShips_Vol1/Materials/GB4_Supercarrier/Fighter/MI_GB4_Fighter_Black.MI_GB4_Fighter_Black")
          (`PrimitiveComponent.SetMaterial` _sm_gb4_supercarrier_fighter_3 0 "/Game/SpaceShips_Vol1/Materials/GB4_Supercarrier/Fighter/MI_GB4_Fighter_Black.MI_GB4_Fighter_Black"))
        (:`0`
          (goto _label))
        (:`1`
          (`PrimitiveComponent.SetMaterial` _sm_gb4_supercarrier 0 "/Game/SpaceShips_Vol1/Materials/GB4_Supercarrier/MI_GB4_SuperCarrier_White.MI_GB4_SuperCarrier_White")
          (`PrimitiveComponent.SetMaterial` _sm_gb4_supercarrier_fighter 0 "/Game/SpaceShips_Vol1/Materials/GB4_Supercarrier/Fighter/MI_GB4_Fighter_White.MI_GB4_Fighter_White")
          (`PrimitiveComponent.SetMaterial` _sm_gb4_supercarrier_fighter_1 0 "/Game/SpaceShips_Vol1/Materials/GB4_Supercarrier/Fighter/MI_GB4_Fighter_White.MI_GB4_Fighter_White")
          (`PrimitiveComponent.SetMaterial` _sm_gb4_supercarrier_fighter_2 0 "/Game/SpaceShips_Vol1/Materials/GB4_Supercarrier/Fighter/MI_GB4_Fighter_White.MI_GB4_Fighter_White")
          (`PrimitiveComponent.SetMaterial` _sm_gb4_supercarrier_fighter_3 0 "/Game/SpaceShips_Vol1/Materials/GB4_Supercarrier/Fighter/MI_GB4_Fighter_White.MI_GB4_Fighter_White"))
        (:`2`
          (`PrimitiveComponent.SetMaterial` _sm_gb4_supercarrier 0 "/Game/SpaceShips_Vol1/Materials/GB4_Supercarrier/MI_GB4_SuperCarrier_Yellow.MI_GB4_SuperCarrier_Yellow")
          (`PrimitiveComponent.SetMaterial` _sm_gb4_supercarrier_fighter 0 "/Game/SpaceShips_Vol1/Materials/GB4_Supercarrier/Fighter/MI_GB4_Fighter_Yellow.MI_GB4_Fighter_Yellow")
          (`PrimitiveComponent.SetMaterial` _sm_gb4_supercarrier_fighter_1 0 "/Game/SpaceShips_Vol1/Materials/GB4_Supercarrier/Fighter/MI_GB4_Fighter_Yellow.MI_GB4_Fighter_Yellow")
          (`PrimitiveComponent.SetMaterial` _sm_gb4_supercarrier_fighter_2 0 "/Game/SpaceShips_Vol1/Materials/GB4_Supercarrier/Fighter/MI_GB4_Fighter_Yellow.MI_GB4_Fighter_Yellow")
          (`PrimitiveComponent.SetMaterial` _sm_gb4_supercarrier_fighter_3 0 "/Game/SpaceShips_Vol1/Materials/GB4_Supercarrier/Fighter/MI_GB4_Fighter_Yellow.MI_GB4_Fighter_Yellow"))
        (:`3`
          (`PrimitiveComponent.SetMaterial` _sm_gb4_supercarrier 0 "/Game/SpaceShips_Vol1/Materials/GB4_Supercarrier/MI_GB4_SuperCarrier_Green.MI_GB4_SuperCarrier_Green")
          (`PrimitiveComponent.SetMaterial` _sm_gb4_supercarrier_fighter 0 "/Game/SpaceShips_Vol1/Materials/GB4_Supercarrier/Fighter/MI_GB4_Fighter_Green.MI_GB4_Fighter_Green")
          (`PrimitiveComponent.SetMaterial` _sm_gb4_supercarrier_fighter_1 0 "/Game/SpaceShips_Vol1/Materials/GB4_Supercarrier/Fighter/MI_GB4_Fighter_Green.MI_GB4_Fighter_Green")
          (`PrimitiveComponent.SetMaterial` _sm_gb4_supercarrier_fighter_2 0 "/Game/SpaceShips_Vol1/Materials/GB4_Supercarrier/Fighter/MI_GB4_Fighter_Green.MI_GB4_Fighter_Green")
          (`PrimitiveComponent.SetMaterial` _sm_gb4_supercarrier_fighter_3 0 "/Game/SpaceShips_Vol1/Materials/GB4_Supercarrier/Fighter/MI_GB4_Fighter_Green.MI_GB4_Fighter_Green"))
        (:`4`
          (`PrimitiveComponent.SetMaterial` _sm_gb4_supercarrier 0 "/Game/SpaceShips_Vol1/Materials/GB4_Supercarrier/MI_GB4_SuperCarrier_Red.MI_GB4_SuperCarrier_Red")
          (`PrimitiveComponent.SetMaterial` _sm_gb4_supercarrier_fighter 0 "/Game/SpaceShips_Vol1/Materials/GB4_Supercarrier/Fighter/MI_GB4_Fighter_Red.MI_GB4_Fighter_Red")
          (`PrimitiveComponent.SetMaterial` _sm_gb4_supercarrier_fighter_1 0 "/Game/SpaceShips_Vol1/Materials/GB4_Supercarrier/Fighter/MI_GB4_Fighter_Red.MI_GB4_Fighter_Red")
          (`PrimitiveComponent.SetMaterial` _sm_gb4_supercarrier_fighter_2 0 "/Game/SpaceShips_Vol1/Materials/GB4_Supercarrier/Fighter/MI_GB4_Fighter_Red.MI_GB4_Fighter_Red")
          (`PrimitiveComponent.SetMaterial` _sm_gb4_supercarrier_fighter_3 0 "/Game/SpaceShips_Vol1/Materials/GB4_Supercarrier/Fighter/MI_GB4_Fighter_Red.MI_GB4_Fighter_Red"))
        (:`5`
          (`PrimitiveComponent.SetMaterial` _sm_gb4_supercarrier 0 "/Game/SpaceShips_Vol1/Materials/GB4_Supercarrier/MI_GB4_SuperCarrier_Blue.MI_GB4_SuperCarrier_Blue")
          (`PrimitiveComponent.SetMaterial` _sm_gb4_supercarrier_fighter 0 "/Game/SpaceShips_Vol1/Materials/GB4_Supercarrier/Fighter/MI_GB4_Fighter_Blue.MI_GB4_Fighter_Blue")
          (`PrimitiveComponent.SetMaterial` _sm_gb4_supercarrier_fighter_1 0 "/Game/SpaceShips_Vol1/Materials/GB4_Supercarrier/Fighter/MI_GB4_Fighter_Blue.MI_GB4_Fighter_Blue")
          (`PrimitiveComponent.SetMaterial` _sm_gb4_supercarrier_fighter_2 0 "/Game/SpaceShips_Vol1/Materials/GB4_Supercarrier/Fighter/MI_GB4_Fighter_Blue.MI_GB4_Fighter_Blue")
          (`PrimitiveComponent.SetMaterial` _sm_gb4_supercarrier_fighter_3 0 "/Game/SpaceShips_Vol1/Materials/GB4_Supercarrier/Fighter/MI_GB4_Fighter_Blue.MI_GB4_Fighter_Blue"))))))