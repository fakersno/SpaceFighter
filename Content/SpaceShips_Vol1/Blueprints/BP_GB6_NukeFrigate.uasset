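; Nuke frigate ship Blueprint that fires six missiles from behind hinged doors when FireMissiles is called.
; A Sequence with staggered delays calls Launch on each child-actor missile and starts its own Timeline.
; Each Timeline pitches a door open and pushes the missile along local Z by incremental offsets, then hides it when finished.
; The construction script applies a Color-selected material to hull and doors.
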(event `self.ReceiveBeginPlay`)

(event `FireMissiles`
  (bind _bp_nukefrigate_missile1 (`self.BP_NukeFrigate_Missile1`))
  (bind _bp_nukefrigate_missile2 (`self.BP_NukeFrigate_Missile2`))
  (bind _bp_nukefrigate_missile3 (`self.BP_NukeFrigate_Missile3`))
  (bind _bp_nukefrigate_missile4 (`self.BP_NukeFrigate_Missile4`))
  (bind _bp_nukefrigate_missile5 (`self.BP_NukeFrigate_Missile5`))
  (bind _bp_nukefrigate_missile6 (`self.BP_NukeFrigate_Missile6`))
  (`|ExecutionSequence`
    (:`then_0`
      (`self.Launch` _bp_nukefrigate_missile1)
      (bind (_direction _door _missile) (`Timeline|Timeline_0` :!via `PlayFromStart`)
        (:`Update`
          (`self.DoorOpening` (`self.Door1`) _door)
          (`self.MissileLaunch` _bp_nukefrigate_missile1 _missile))
        (:`Finished`
          (`SceneComponent.SetHiddenInGame` _bp_nukefrigate_missile1 true false))))
    (:`then_1`
      (`KismetSystemLibrary.Delay` 0.5)
      (`self.Launch` _bp_nukefrigate_missile2)
      (bind (_direction_2 _door_2 _missile_2) (`Timeline|Timeline_1`)
        (:`Update`
          (`self.DoorOpening` (`self.Door2`) _door_2)
          (`self.MissileLaunch` _bp_nukefrigate_missile2 _missile_2))
        (:`Finished`
          (`SceneComponent.SetHiddenInGame` _bp_nukefrigate_missile2 true false))))
    (:`then_2`
      (`KismetSystemLibrary.Delay` 1.0)
      (`self.Launch` _bp_nukefrigate_missile3)
      (bind (_direction_3 _door_3 _missile_3) (`Timeline|Timeline_2` :!via `PlayFromStart`)
        (:`Update`
          (`self.DoorOpening` (`self.Door3`) _door_3)
          (`self.MissileLaunch` _bp_nukefrigate_missile3 _missile_3))
        (:`Finished`
          (`SceneComponent.SetHiddenInGame` _bp_nukefrigate_missile3 true false))))
    (:`then_3`
      (`KismetSystemLibrary.Delay` 1.5)
      (`self.Launch` _bp_nukefrigate_missile4)
      (bind (_direction_4 _door_4 _missile_4) (`Timeline|Timeline_3` :!via `PlayFromStart`)
        (:`Update`
          (`self.DoorOpening` (`self.Door4`) _door_4)
          (`self.MissileLaunch` _bp_nukefrigate_missile4 _missile_4))
        (:`Finished`
          (`SceneComponent.SetHiddenInGame` _bp_nukefrigate_missile4 true false))))
    (:`then_4`
      (`KismetSystemLibrary.Delay` 2.0)
      (`self.Launch` _bp_nukefrigate_missile5)
      (bind (_direction_5 _door_5 _missile_5) (`Timeline|Timeline_4` :!via `PlayFromStart`)
        (:`Update`
          (`self.DoorOpening` (`self.Door5`) _door_5)
          (`self.MissileLaunch` _bp_nukefrigate_missile5 _missile_5))
        (:`Finished`
          (`SceneComponent.SetHiddenInGame` _bp_nukefrigate_missile5 true false))))
    (:`then_5`
      (`KismetSystemLibrary.Delay` 2.5)
      (`self.Launch` _bp_nukefrigate_missile6)
      (bind (_direction_6 _door_6 _missile_6) (`Timeline|Timeline_5` :!via `PlayFromStart`)
        (:`Update`
          (`self.DoorOpening` (`self.Door6`) _door_6)
          (`self.MissileLaunch` _bp_nukefrigate_missile6 _missile_6))
        (:`Finished`
          (`SceneComponent.SetHiddenInGame` _bp_nukefrigate_missile6 true false))))))

(fn `UserConstructionScript`
  (bind _sm_gb6_dreadnought (`self.SM_GB6_Dreadnought`))
  (switch `int` (`self.Color`)
    (:`Default`
      (`PrimitiveComponent.SetMaterial` _sm_gb6_dreadnought 0 "/Game/SpaceShips_Vol1/Materials/GB5_NukeFrigate/MI_GB5_NukeFrigate_Black.MI_GB5_NukeFrigate_Black" :!label _label)
      (`PrimitiveComponent.SetMaterial` (`self.Door4`) 0 "/Game/SpaceShips_Vol1/Materials/GB5_NukeFrigate/MI_GB5_NukeFrigate_Black.MI_GB5_NukeFrigate_Black")
      (`PrimitiveComponent.SetMaterial` (`self.Door2`) 0 "/Game/SpaceShips_Vol1/Materials/GB5_NukeFrigate/MI_GB5_NukeFrigate_Black.MI_GB5_NukeFrigate_Black")
      (`PrimitiveComponent.SetMaterial` (`self.Door5`) 0 "/Game/SpaceShips_Vol1/Materials/GB5_NukeFrigate/MI_GB5_NukeFrigate_Black.MI_GB5_NukeFrigate_Black")
      (`PrimitiveComponent.SetMaterial` (`self.Door3`) 0 "/Game/SpaceShips_Vol1/Materials/GB5_NukeFrigate/MI_GB5_NukeFrigate_Black.MI_GB5_NukeFrigate_Black")
      (`PrimitiveComponent.SetMaterial` (`self.Door6`) 0 "/Game/SpaceShips_Vol1/Materials/GB5_NukeFrigate/MI_GB5_NukeFrigate_Black.MI_GB5_NukeFrigate_Black")
      (`PrimitiveComponent.SetMaterial` (`self.Door1`) 0 "/Game/SpaceShips_Vol1/Materials/GB5_NukeFrigate/MI_GB5_NukeFrigate_Black.MI_GB5_NukeFrigate_Black"))
    (:`0`
      (goto _label))
    (:`1`
      (`PrimitiveComponent.SetMaterial` _sm_gb6_dreadnought 0 "/Game/SpaceShips_Vol1/Materials/GB5_NukeFrigate/MI_GB5_NukeFrigate_White.MI_GB5_NukeFrigate_White")
      (`PrimitiveComponent.SetMaterial` (`self.Door4`) 0 "/Game/SpaceShips_Vol1/Materials/GB5_NukeFrigate/MI_GB5_NukeFrigate_White.MI_GB5_NukeFrigate_White")
      (`PrimitiveComponent.SetMaterial` (`self.Door2`) 0 "/Game/SpaceShips_Vol1/Materials/GB5_NukeFrigate/MI_GB5_NukeFrigate_White.MI_GB5_NukeFrigate_White")
      (`PrimitiveComponent.SetMaterial` (`self.Door5`) 0 "/Game/SpaceShips_Vol1/Materials/GB5_NukeFrigate/MI_GB5_NukeFrigate_White.MI_GB5_NukeFrigate_White")
      (`PrimitiveComponent.SetMaterial` (`self.Door3`) 0 "/Game/SpaceShips_Vol1/Materials/GB5_NukeFrigate/MI_GB5_NukeFrigate_White.MI_GB5_NukeFrigate_White")
      (`PrimitiveComponent.SetMaterial` (`self.Door6`) 0 "/Game/SpaceShips_Vol1/Materials/GB5_NukeFrigate/MI_GB5_NukeFrigate_White.MI_GB5_NukeFrigate_White")
      (`PrimitiveComponent.SetMaterial` (`self.Door1`) 0 "/Game/SpaceShips_Vol1/Materials/GB5_NukeFrigate/MI_GB5_NukeFrigate_White.MI_GB5_NukeFrigate_White"))
    (:`2`
      (`PrimitiveComponent.SetMaterial` _sm_gb6_dreadnought 0 "/Game/SpaceShips_Vol1/Materials/GB5_NukeFrigate/MI_GB5_NukeFrigate_Yellow.MI_GB5_NukeFrigate_Yellow")
      (`PrimitiveComponent.SetMaterial` (`self.Door4`) 0 "/Game/SpaceShips_Vol1/Materials/GB5_NukeFrigate/MI_GB5_NukeFrigate_Yellow.MI_GB5_NukeFrigate_Yellow")
      (`PrimitiveComponent.SetMaterial` (`self.Door2`) 0 "/Game/SpaceShips_Vol1/Materials/GB5_NukeFrigate/MI_GB5_NukeFrigate_Yellow.MI_GB5_NukeFrigate_Yellow")
      (`PrimitiveComponent.SetMaterial` (`self.Door5`) 0 "/Game/SpaceShips_Vol1/Materials/GB5_NukeFrigate/MI_GB5_NukeFrigate_Yellow.MI_GB5_NukeFrigate_Yellow")
      (`PrimitiveComponent.SetMaterial` (`self.Door3`) 0 "/Game/SpaceShips_Vol1/Materials/GB5_NukeFrigate/MI_GB5_NukeFrigate_Yellow.MI_GB5_NukeFrigate_Yellow")
      (`PrimitiveComponent.SetMaterial` (`self.Door6`) 0 "/Game/SpaceShips_Vol1/Materials/GB5_NukeFrigate/MI_GB5_NukeFrigate_Yellow.MI_GB5_NukeFrigate_Yellow")
      (`PrimitiveComponent.SetMaterial` (`self.Door1`) 0 "/Game/SpaceShips_Vol1/Materials/GB5_NukeFrigate/MI_GB5_NukeFrigate_Yellow.MI_GB5_NukeFrigate_Yellow"))
    (:`3`
      (`PrimitiveComponent.SetMaterial` _sm_gb6_dreadnought 0 "/Game/SpaceShips_Vol1/Materials/GB5_NukeFrigate/MI_GB5_NukeFrigate_Green.MI_GB5_NukeFrigate_Green")
      (`PrimitiveComponent.SetMaterial` (`self.Door4`) 0 "/Game/SpaceShips_Vol1/Materials/GB5_NukeFrigate/MI_GB5_NukeFrigate_Green.MI_GB5_NukeFrigate_Green")
      (`PrimitiveComponent.SetMaterial` (`self.Door2`) 0 "/Game/SpaceShips_Vol1/Materials/GB5_NukeFrigate/MI_GB5_NukeFrigate_Green.MI_GB5_NukeFrigate_Green")
      (`PrimitiveComponent.SetMaterial` (`self.Door5`) 0 "/Game/SpaceShips_Vol1/Materials/GB5_NukeFrigate/MI_GB5_NukeFrigate_Green.MI_GB5_NukeFrigate_Green")
      (`PrimitiveComponent.SetMaterial` (`self.Door3`) 0 "/Game/SpaceShips_Vol1/Materials/GB5_NukeFrigate/MI_GB5_NukeFrigate_Green.MI_GB5_NukeFrigate_Green")
      (`PrimitiveComponent.SetMaterial` (`self.Door6`) 0 "/Game/SpaceShips_Vol1/Materials/GB5_NukeFrigate/MI_GB5_NukeFrigate_Green.MI_GB5_NukeFrigate_Green")
      (`PrimitiveComponent.SetMaterial` (`self.Door1`) 0 "/Game/SpaceShips_Vol1/Materials/GB5_NukeFrigate/MI_GB5_NukeFrigate_Green.MI_GB5_NukeFrigate_Green"))
    (:`4`
      (`PrimitiveComponent.SetMaterial` _sm_gb6_dreadnought 0 "/Game/SpaceShips_Vol1/Materials/GB5_NukeFrigate/MI_GB5_NukeFrigate_Red.MI_GB5_NukeFrigate_Red")
      (`PrimitiveComponent.SetMaterial` (`self.Door4`) 0 "/Game/SpaceShips_Vol1/Materials/GB5_NukeFrigate/MI_GB5_NukeFrigate_Red.MI_GB5_NukeFrigate_Red")
      (`PrimitiveComponent.SetMaterial` (`self.Door2`) 0 "/Game/SpaceShips_Vol1/Materials/GB5_NukeFrigate/MI_GB5_NukeFrigate_Red.MI_GB5_NukeFrigate_Red")
      (`PrimitiveComponent.SetMaterial` (`self.Door5`) 0 "/Game/SpaceShips_Vol1/Materials/GB5_NukeFrigate/MI_GB5_NukeFrigate_Red.MI_GB5_NukeFrigate_Red")
      (`PrimitiveComponent.SetMaterial` (`self.Door3`) 0 "/Game/SpaceShips_Vol1/Materials/GB5_NukeFrigate/MI_GB5_NukeFrigate_Red.MI_GB5_NukeFrigate_Red")
      (`PrimitiveComponent.SetMaterial` (`self.Door6`) 0 "/Game/SpaceShips_Vol1/Materials/GB5_NukeFrigate/MI_GB5_NukeFrigate_Red.MI_GB5_NukeFrigate_Red")
      (`PrimitiveComponent.SetMaterial` (`self.Door1`) 0 "/Game/SpaceShips_Vol1/Materials/GB5_NukeFrigate/MI_GB5_NukeFrigate_Red.MI_GB5_NukeFrigate_Red"))
    (:`5`
      (`PrimitiveComponent.SetMaterial` _sm_gb6_dreadnought 0 "/Game/SpaceShips_Vol1/Materials/GB5_NukeFrigate/MI_GB5_NukeFrigate_Blue.MI_GB5_NukeFrigate_Blue")
      (`PrimitiveComponent.SetMaterial` (`self.Door4`) 0 "/Game/SpaceShips_Vol1/Materials/GB5_NukeFrigate/MI_GB5_NukeFrigate_Blue.MI_GB5_NukeFrigate_Blue")
      (`PrimitiveComponent.SetMaterial` (`self.Door2`) 0 "/Game/SpaceShips_Vol1/Materials/GB5_NukeFrigate/MI_GB5_NukeFrigate_Blue.MI_GB5_NukeFrigate_Blue")
      (`PrimitiveComponent.SetMaterial` (`self.Door5`) 0 "/Game/SpaceShips_Vol1/Materials/GB5_NukeFrigate/MI_GB5_NukeFrigate_Blue.MI_GB5_NukeFrigate_Blue")
      (`PrimitiveComponent.SetMaterial` (`self.Door3`) 0 "/Game/SpaceShips_Vol1/Materials/GB5_NukeFrigate/MI_GB5_NukeFrigate_Blue.MI_GB5_NukeFrigate_Blue")
      (`PrimitiveComponent.SetMaterial` (`self.Door6`) 0 "/Game/SpaceShips_Vol1/Materials/GB5_NukeFrigate/MI_GB5_NukeFrigate_Blue.MI_GB5_NukeFrigate_Blue")
      (`PrimitiveComponent.SetMaterial` (`self.Door1`) 0 "/Game/SpaceShips_Vol1/Materials/GB5_NukeFrigate/MI_GB5_NukeFrigate_Blue.MI_GB5_NukeFrigate_Blue"))))