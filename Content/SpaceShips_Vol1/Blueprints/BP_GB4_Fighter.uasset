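; BP_GB4_Fighter is a configurable GB4 fighter spaceship prop from the SpaceShips_Vol1 content, with no active gameplay logic.
; Its Construction Script shows or hides the two rocket flare meshes in game from the RocketFlares flag.
; It also switches on Color to apply one of six paint material instances to the hull mesh's first material slot.
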(fn `UserConstructionScript`
  (bind _sm_gb4_fighter (`self.SM_GB4_Fighter`))
  (`SceneComponent.SetHiddenInGame` (`self.SM_RocketFlare_2`) (not (`self.RocketFlares`)) false)
  (`SceneComponent.SetHiddenInGame` (`self.SM_RocketFlare_1`) (not (`self.RocketFlares`)) false)
  (switch `int` (`self.Color`)
    (:`0`
      (`PrimitiveComponent.SetMaterial` _sm_gb4_fighter 0 "/Game/SpaceShips_Vol1/Materials/GB4_Supercarrier/Fighter/MI_GB4_Fighter_Black.MI_GB4_Fighter_Black"))
    (:`1`
      (`PrimitiveComponent.SetMaterial` _sm_gb4_fighter 0 "/Game/SpaceShips_Vol1/Materials/GB4_Supercarrier/Fighter/MI_GB4_Fighter_White.MI_GB4_Fighter_White"))
    (:`2`
      (`PrimitiveComponent.SetMaterial` _sm_gb4_fighter 0 "/Game/SpaceShips_Vol1/Materials/GB4_Supercarrier/Fighter/MI_GB4_Fighter_Yellow.MI_GB4_Fighter_Yellow"))
    (:`3`
      (`PrimitiveComponent.SetMaterial` _sm_gb4_fighter 0 "/Game/SpaceShips_Vol1/Materials/GB4_Supercarrier/Fighter/MI_GB4_Fighter_Green.MI_GB4_Fighter_Green"))
    (:`4`
      (`PrimitiveComponent.SetMaterial` _sm_gb4_fighter 0 "/Game/SpaceShips_Vol1/Materials/GB4_Supercarrier/Fighter/MI_GB4_Fighter_Red.MI_GB4_Fighter_Red"))
    (:`5`
      (`PrimitiveComponent.SetMaterial` _sm_gb4_fighter 0 "/Game/SpaceShips_Vol1/Materials/GB4_Supercarrier/Fighter/MI_GB4_Fighter_Blue.MI_GB4_Fighter_Blue"))))