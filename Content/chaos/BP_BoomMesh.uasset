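; BP_BoomMesh is a destructible asteroid that explodes and shatters when damage depletes its Health.
; Any damage taken lowers Health, and at zero or below it spawns an oversized explosion emitter and calls Broke.
; Broke swaps the intact static mesh for a simulating Chaos Geometry Collection, toggling visibility, collision and physics.
; After a brief delay it spawns BP_BoomFied at the Scene transform, apparently a field to scatter the pieces.
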(event `self.ReceiveBeginPlay`
  (`self.EnableInput` (`GameplayStatics.GetPlayerController` 0))
  (add `self.OnTakeAnyDamage` (delegate `RescetDamage`)))

(event `RescetDamage` :!signature `self.OnTakeAnyDamage`
  (params (DamagedActor :type "Actor Object Reference") (Damage :type "Float (single-precision)") (DamageType :type "DamageType Object Reference") (InstigatedBy :type "Controller Object Reference") (DamageCauser :type "Actor Object Reference"))
  (`KismetSystemLibrary.PrintString` "Hello")
  (bind _output_get (set `self.Health` (- (`self.Health`) Damage)))
  (if (<= _output_get 0.0)
    (`GameplayStatics.SpawnEmitterAtLocation` "/Game/PolygonSciFiSpace/FX/FX_Explosion.FX_Explosion" (`SceneComponent.K2_GetComponentLocation` (`self.Scene`)) (struct) (100.0 100.0 100.0) false)
    (`self.Broke`)))

(event `Broke`
  (bind _geometrycollection (`self.GeometryCollection`))
  (bind _sm_env_asteroid_02 (`self.SM_Env_Asteroid_02`))
  (`SceneComponent.SetHiddenInGame` _sm_env_asteroid_02 true false)
  (`PrimitiveComponent.SetCollisionEnabled` _sm_env_asteroid_02 "NoCollision")
  (`PrimitiveComponent.SetSimulatePhysics` _sm_env_asteroid_02 (`PrimitiveComponent.K2_IsCollisionEnabled` _sm_env_asteroid_02))
  (`SceneComponent.SetHiddenInGame` _geometrycollection false false)
  (`PrimitiveComponent.SetCollisionEnabled` _geometrycollection "QueryAndPhysics")
  (`PrimitiveComponent.SetSimulatePhysics` _geometrycollection (`PrimitiveComponent.K2_IsCollisionEnabled` _geometrycollection))
  (`KismetSystemLibrary.Delay` 0.05)
  (`|SpawnActorFromClass` "/Game/chaos/BP_BoomFied.BP_BoomFied_C" (`SceneComponent.K2_GetComponentToWorld` (`self.Scene`)) "Undefined" "OverrideRootScale" null null))

(fn `UserConstructionScript`)