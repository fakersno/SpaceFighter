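; BP_BoomFied is a Chaos field actor that produces a one-shot explosion to break and scatter destructible objects.
; On BeginPlay it applies external cluster strain through a radial falloff sized and centred on its Sphere component.
; It then applies a radial-vector linear force, culled outside that same sphere, to push the pieces outward.
; The actor destroys itself after a short delay.
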(event `self.ReceiveBeginPlay`
  (bind _fieldsystemcomponent (`self.FieldSystemComponent`))
  (bind _sphere (`self.Sphere`))
  (bind _returnvalue (`SceneComponent.K2_GetComponentLocation` _sphere))
  (bind _returnvalue_2 (`RadialFalloff.SetRadialFalloff` (`self.RadialFalloff`) (`self.Radial Falloff`) 0.0 1.0 0.0 (`SphereComponent.GetScaledSphereRadius` _sphere) _returnvalue "Field_FallOff_None"))
  (`FieldSystemComponent.ApplyPhysicsField` _fieldsystemcomponent true "Field_ExternalClusterStrain" null _returnvalue_2)
  (`FieldSystemComponent.ApplyPhysicsField` _fieldsystemcomponent true "Field_LinearForce" null (`CullingField.SetCullingField` (`self.CullingField`) _returnvalue_2 (`RadialVector.SetRadialVector` (`self.RadialVector`) (`self.RadialVector `) _returnvalue) "Field_Culling_Outside"))
  (`KismetSystemLibrary.Delay` 5.0)
  (`self.K2_DestroyActor`))

(fn `UserConstructionScript`)