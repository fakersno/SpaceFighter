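; Game mode that sets up local multiplayer, with one player per BP_PlayerStart in the level.
; On BeginPlay it creates an extra local player and controller for each start beyond the first.
; For each start tagged "Player" plus its own array index, it spawns a BP_TypeA there, possesses it with that player's controller and adds a reticle widget to that player's screen.
; Starts whose tag differs from their array position are skipped.
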(event `self.ReceiveBeginPlay`
  (bind _outactors (`GameplayStatics.GetAllActorsOfClass` "/Game/BP/PlayerStart/BP_PlayerStart.BP_PlayerStart_C"))
  (for _index (range 1 (`KismetArrayLibrary.Array_Length` _outactors))
    (`GameplayStatics.CreatePlayer` _index))
  (for (_array_element _array_index) _outactors
    (if (== (`PlayerStart.PlayerStartTag` _array_element) (`KismetStringLibrary.Concat_StrStr` "Player" (`KismetStringLibrary.Conv_IntToString` _array_index)))
      (set `self.PlayerIndex` _array_index)
      (bind _returnvalue (`|SpawnActorFromClass` "/Game/BP/Fighters/BP_TypeA.BP_TypeA_C" (`self.GetTransform` _array_element) "Undefined" "OverrideRootScale" null null))
      (`Controller.Possess` (`GameplayStatics.GetPlayerController` (`self.PlayerIndex`)) _returnvalue)
      (bind _returnvalue_2 (`|CreateWidget` "/Game/BP/UMG/UMG_WidgetReticle.UMG_WidgetReticle_C" (`GameplayStatics.GetPlayerController` (`self.PlayerIndex`))))
      (`UserWidget.AddToPlayerScreen` _returnvalue_2 0))))

(fn `UserConstructionScript`)