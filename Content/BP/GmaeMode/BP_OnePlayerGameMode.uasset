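; Game mode that sets up local players on BeginPlay, one per BP_PlayerStart in the level despite its OnePlayer name.
; It creates the extra local players, then spawns and possesses a BP_Fighter2 at each start tagged "Player" plus its array index.
; Each fighter is linked to its BP_FighterController and a per-player UMG_WidgetReticle added to that player's screen.
; Starts whose tag does not match their position in the actor array get no fighter.
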(event `self.ReceiveBeginPlay`
  (bind _returnvalue (`GameplayStatics.GetPlayerController` (`self.PlayerIndex`)))
  (bind _returnvalue_2 (`GameplayStatics.GetPlayerController` (`self.PlayerIndex`)))
  (bind _outactors (`GameplayStatics.GetAllActorsOfClass` "/Game/BP/PlayerStart/BP_PlayerStart.BP_PlayerStart_C"))
  (for _index (range 1 (`KismetArrayLibrary.Array_Length` _outactors))
    (`GameplayStatics.CreatePlayer` _index))
  (for (_array_element _array_index) _outactors
    (if (== (`PlayerStart.PlayerStartTag` _array_element) (`KismetStringLibrary.Concat_StrStr` "Player" (`KismetStringLibrary.Conv_IntToString` _array_index)))
      (set `self.PlayerIndex` _array_index)
      (bind _returnvalue_3 (`|SpawnActorFromClass` "/Game/BP/Fighters/BP_Fighter2.BP_Fighter2_C" (`self.GetTransform` _array_element) "AlwaysSpawn" "OverrideRootScale" _returnvalue null))
      (bind _asbp_fighter_controller (cast `/Game/BP/Controller/BP_FighterController` _returnvalue))
      (set `/Game/BP/Fighters/BP_TypeA.MyPlayercontroller` _asbp_fighter_controller _returnvalue_3)
      (`Controller.Possess` _returnvalue _returnvalue_3)
      (bind _asbp_fighter_controller_2 (cast `/Game/BP/Controller/BP_FighterController` _returnvalue))
      (bind _returnvalue_4 (`|CreateWidget` "/Game/BP/UMG/UMG_WidgetReticle.UMG_WidgetReticle_C" _returnvalue_2))
      (set `/Game/BP/Fighters/BP_TypeA.PlayerWidget` _returnvalue_4 _returnvalue_3)
      (bind _asbp_fighter_controller_3 (cast `/Game/BP/Controller/BP_FighterController` _returnvalue_2))
      (set `/Game/BP/UMG/UMG_WidgetReticle.Owner` _asbp_fighter_controller_3 _returnvalue_4)
      (set `/Game/BP/Controller/BP_FighterController.UMGMain` _returnvalue_4 _asbp_fighter_controller_2)
      (`UserWidget.AddToPlayerScreen` _returnvalue_4 0))))

(fn `UserConstructionScript`)