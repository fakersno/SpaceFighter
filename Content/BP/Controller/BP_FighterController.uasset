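; Player controller for two local fighter pilots, routing input to the BP_TypeA pawns of players 0 and 1.
; Per-player axes and keys drive thrust, turn, roll, vertical adjustment, firing and camera toggling, with mouse X also feeding player 0's roll.
; Holding LookAround lets the mouse orbit player 0's spring-arm camera and hides that HUD widget.
; ReturnMenuMap pauses and shows a return-menu widget with UI-only input.
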(event `InputAxis|Thrust0`
  (params (AxisValue :type "Float (single-precision)"))
  (bind _asbp_type_a (cast `/Game/BP/Fighters/BP_TypeA` (`GameplayStatics.GetPlayerPawn` 0)))
  (`/Game/BP/Fighters/BP_TypeA.Thrust` _asbp_type_a AxisValue))

(event `InputAxis|Thrust1`
  (params (AxisValue :type "Float (single-precision)"))
  (bind _asbp_type_a (cast `/Game/BP/Fighters/BP_TypeA` (`GameplayStatics.GetPlayerPawn` 1)))
  (`/Game/BP/Fighters/BP_TypeA.Thrust` _asbp_type_a AxisValue))

(event `Key|C`
  (params (Key :type "Key Structure"))
  (:`Pressed`
    (bind _asbp_type_a (cast `/Game/BP/Fighters/BP_TypeA` (`GameplayStatics.GetPlayerPawn` 0)))
    (`/Game/BP/Fighters/BP_TypeA.Toggle Cmaera` _asbp_type_a)))

(event `Key|Decimal`
  (params (Key :type "Key Structure"))
  (:`Pressed`
    (bind _asbp_type_a (cast `/Game/BP/Fighters/BP_TypeA` (`GameplayStatics.GetPlayerPawn` 1)))
    (`/Game/BP/Fighters/BP_TypeA.Toggle Cmaera` _asbp_type_a)))

(event `InputAction|Fire0`
  (params (Key :type "Key Structure"))
  (bind _returnvalue (`GameplayStatics.GetPlayerPawn` 0))
  (:`Pressed`
    (bind _asbp_type_a (cast `/Game/BP/Fighters/BP_TypeA` _returnvalue))
    (`/Game/BP/Fighters/BP_TypeA.StartFire` _asbp_type_a))
  (:`Released`
    (bind _asbp_type_a_2 (cast `/Game/BP/Fighters/BP_TypeA` _returnvalue))
    (`/Game/BP/Fighters/BP_TypeA.StopFire` _asbp_type_a)
    (`/Game/BP/Fighters/BP_TypeA.StopFire` _asbp_type_a_2)))

(event `InputAction|Fire1`
  (params (Key :type "Key Structure"))
  (bind _returnvalue (`GameplayStatics.GetPlayerPawn` 1))
  (:`Pressed`
    (bind _asbp_type_a (cast `/Game/BP/Fighters/BP_TypeA` _returnvalue))
    (`/Game/BP/Fighters/BP_TypeA.StartFire` _asbp_type_a))
  (:`Released`
    (bind _asbp_type_a_2 (cast `/Game/BP/Fighters/BP_TypeA` _returnvalue))
    (`/Game/BP/Fighters/BP_TypeA.StopFire` _asbp_type_a)
    (`/Game/BP/Fighters/BP_TypeA.StopFire` _asbp_type_a_2)))

(event `InputAxis|AdjustUp0`
  (params (AxisValue :type "Float (single-precision)"))
  (bind _asbp_type_a (cast `/Game/BP/Fighters/BP_TypeA` (`GameplayStatics.GetPlayerPawn` 0)))
  (`/Game/BP/Fighters/BP_TypeA.AdjustUp` _asbp_type_a AxisValue))

(event `InputAxis|AdjustUp1`
  (params (AxisValue :type "Float (single-precision)"))
  (bind _asbp_type_a (cast `/Game/BP/Fighters/BP_TypeA` (`GameplayStatics.GetPlayerPawn` 1)))
  (`/Game/BP/Fighters/BP_TypeA.AdjustUp` _asbp_type_a AxisValue))

(event `InputAxis|LookUp0`
  (params (AxisValue :type "Float (single-precision)"))
  (if (not (`self.LookAround`))
    (bind _asbp_type_a (cast `/Game/BP/Fighters/BP_TypeA` (`GameplayStatics.GetPlayerPawn` 0)))
    (`/Game/BP/Fighters/BP_TypeA.LookUp` _asbp_type_a AxisValue)))

(event `InputAxis|Turn0`
  (params (AxisValue :type "Float (single-precision)"))
  (bind _asbp_type_a (cast `/Game/BP/Fighters/BP_TypeA` (`GameplayStatics.GetPlayerPawn` 0)))
  (`/Game/BP/Fighters/BP_TypeA.Turn` _asbp_type_a AxisValue))

(event `InputAxis|Turn1`
  (params (AxisValue :type "Float (single-precision)"))
  (bind _asbp_type_a (cast `/Game/BP/Fighters/BP_TypeA` (`GameplayStatics.GetPlayerPawn` 1)))
  (`/Game/BP/Fighters/BP_TypeA.Turn` _asbp_type_a AxisValue))

(event `InputAxis|Roll0`
  (params (AxisValue :type "Float (single-precision)"))
  (bind _asbp_type_a (cast `/Game/BP/Fighters/BP_TypeA` (`GameplayStatics.GetPlayerPawn` 0) :!label _label))
  (`/Game/BP/Fighters/BP_TypeA.Roll` _asbp_type_a (`KismetMathLibrary.FClamp` (+ AxisValue (stale `InputAxis|MouseX` _output_get)) -1.0)))

(event `InputAxis|MouseX`
  (params (AxisValue :type "Float (single-precision)"))
  (if (not (`self.LookAround`))
    (bind _output_get (set `self.Axis Value` AxisValue))
    (goto _label)))

(event `InputAxis|Roll1`
  (params (AxisValue :type "Float (single-precision)"))
  (bind _asbp_type_a (cast `/Game/BP/Fighters/BP_TypeA` (`GameplayStatics.GetPlayerPawn` 1)))
  (`/Game/BP/Fighters/BP_TypeA.Roll` _asbp_type_a AxisValue))

(event `InputAction|ChangeWeapon0`
  (params (Key :type "Key Structure")))

(event `InputAction|ChangeWeapon1`
  (params (Key :type "Key Structure")))

(event `InputAction|LookAround`
  (params (Key :type "Key Structure"))
  (:`Pressed`
    (set `self.LookAround` true)
    (bind _asbp_type_a (cast `/Game/BP/Fighters/BP_TypeA` (`GameplayStatics.GetPlayerPawn` 0)))
    (set `SpringArmComponent.bUsePawnControlRotation` true (`/Game/BP/Fighters/BP_TypeA.SpringArm` _asbp_type_a))
    (bind _playerwidget (`/Game/BP/Fighters/BP_TypeA.PlayerWidget` _asbp_type_a))
    (`/Engine/EditorBlueprintResources/StandardMacros.IsValid` _playerwidget
      (:`Is Valid`
        (`Widget.SetVisibility` _playerwidget "Hidden"))))
  (:`Released`
    (set `self.LookAround` false)
    (bind _asbp_type_a_2 (cast `/Game/BP/Fighters/BP_TypeA` (`GameplayStatics.GetPlayerPawn` 0)))
    (set `SpringArmComponent.bUsePawnControlRotation` false (`/Game/BP/Fighters/BP_TypeA.SpringArm` _asbp_type_a_2))
    (bind _playerwidget_2 (`/Game/BP/Fighters/BP_TypeA.PlayerWidget` _asbp_type_a_2))
    (`/Engine/EditorBlueprintResources/StandardMacros.IsValid` _playerwidget_2
      (:`Is Valid`
        (`Widget.SetVisibility` _playerwidget_2 "Visible")))))

(event `InputAction|ReturnMenuMap`
  (params (Key :type "Key Structure"))
  (bind _returnumg (`self.ReturnUMG`))
  (:`Pressed`
    (`GameplayStatics.SetGamePaused` true)
    (if (== _returnumg null)
      (bind _returnvalue (`|CreateWidget` "/Game/BP/UMG/UMG_ReturnMenu.UMG_ReturnMenu_C"))
      (bind _output_get (set `self.ReturnUMG` _returnvalue))
      (`UserWidget.AddToViewport` _output_get 0)
      (set `self.bShowMouseCursor` true)
      (`WidgetBlueprintLibrary.SetInputMode_UIOnlyEx` (`GameplayStatics.GetPlayerController` 0) null "LockAlways")
      (else
        (`Widget.SetVisibility` _returnumg "Visible")
        (set `self.bShowMouseCursor` true)
        (`WidgetBlueprintLibrary.SetInputMode_UIOnlyEx` (`GameplayStatics.GetPlayerController` 0) null "LockAlways")))))

(event `InputAxis|MouseX`
  (params (AxisValue :type "Float (single-precision)"))
  (if (`self.LookAround`)
    (`Pawn.AddControllerYawInput` (`GameplayStatics.GetPlayerPawn` 0) (* AxisValue -1.0))))

(event `InputAxis|MouseY`
  (params (AxisValue :type "Float (single-precision)"))
  (if (`self.LookAround`)
    (`Pawn.AddControllerPitchInput` (`GameplayStatics.GetPlayerPawn` 0) (* AxisValue -1.0))))

(fn `UserConstructionScript`)