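; Turret that picks a random BP_TypeA actor inside its sphere range, tracks it and fires BP_Projectile at it.
; Gated per-frame Delay loops, used instead of Tick, yaw the platform and pitch the clamped cannon toward the target, or ease both back to rest without one.
; Once aligned, it fires after a delay if a visibility trace hits a BP_TypeA, pausing to reload when ammo runs out.
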(event `Shoot`
  (if (`self.ShootingPossible`)
    (`KismetSystemLibrary.Delay` (`self.ShootDelay`))
    (if (> (`self.Ammo`) 0)
      (`/Engine/EditorBlueprintResources/StandardMacros.DecrementInt` (`self.Ammo`)
        (:`  `
          (bind _outhit (`KismetSystemLibrary.LineTraceSingle` (`self.K2_GetActorLocation`) (`self.TargetLocation`) "TraceTypeQuery1"))
          (bind _asbp_type_a (cast `/Game/BP/Fighters/BP_TypeA` (`.HitActor` (`GameplayStatics.BreakHitResult` _outhit))))
          (`/Engine/EditorBlueprintResources/StandardMacros.IsValid` _asbp_type_a
            (:`Is Valid`
              (`|SpawnActorFromClass` "/Game/BP/Weaopn/BP_Projectile.BP_Projectile_C" (`KismetMathLibrary.MakeTransform` (`SceneComponent.K2_GetComponentLocation` (`self.Arrow`)) (`KismetMathLibrary.Conv_VectorToRotator` (`SceneComponent.GetForwardVector` (`self.CannonMesh`)))) "Undefined" "OverrideRootScale" null null)))))
      (else
        (set `self.ShootingPossible` false)
        (`KismetSystemLibrary.Delay` 5.0)
        (set `self.Ammo` 30)
        (set `self.ShootingPossible` true)
        (`KismetSystemLibrary.PrintString` "sssssssss")))))

(event `self.ReceiveBeginPlay`
  (`self.FindTarget`))

(event `self.Sphere.OnComponentBeginOverlap`
  (params (OverlappedComponent :type "PrimitiveComponent Object Reference") (OtherActor :type "Actor Object Reference") (OtherComp :type "PrimitiveComponent Object Reference") (OtherBodyIndex :type Integer) (bFromSweep :type Boolean) (SweepResult :type "HitResult Structure (by ref)"))
  (bind _asbp_type_a (cast `/Game/BP/Fighters/BP_TypeA` OtherActor))
  (`KismetArrayLibrary.Array_Add` (`self.TargetRange`) _asbp_type_a)
  (`/Engine/EditorBlueprintResources/StandardMacros.IsValid` (`self.CurrentTarget`)
    (:`Is Not Valid`
      (`self.FindTarget`)
      (set `self.ShootingPossible` true)
      (`KismetSystemLibrary.PrintString` "Hello"))))

(event `self.Sphere.OnComponentEndOverlap`
  (params (OverlappedComponent :type "PrimitiveComponent Object Reference") (OtherActor :type "Actor Object Reference") (OtherComp :type "PrimitiveComponent Object Reference") (OtherBodyIndex :type Integer))
  (bind _targetrange (`self.TargetRange`))
  (bind _asbp_type_a (cast `/Game/BP/Fighters/BP_TypeA` OtherActor))
  (if (`KismetArrayLibrary.Array_Contains` _targetrange _asbp_type_a)
    (`KismetArrayLibrary.Array_RemoveItem` _targetrange _asbp_type_a)
    (if (== _asbp_type_a (`self.CurrentTarget`))
      (set `self.CurrentTarget` null)
      (`self.FindTarget`)
      (set `self.ShootingPossible` false))))

(event `FindTarget`
  (bind _targetrange (`self.TargetRange`))
  (if (`KismetArrayLibrary.Array_IsValidIndex` _targetrange)
    (set `self.CurrentTarget` (`|GetArrayItem` _targetrange (`KismetMathLibrary.RandomIntegerInRange` 0 (`KismetArrayLibrary.Array_LastIndex` _targetrange))))
    (`self.StartAiming`)
    (else
      (`self.BeginReset`))))

(event `ContinueAiming`
  (bind _turretaimingspeed (`self.TurretAimingSpeed`))
  (bind _currenttarget (`self.CurrentTarget`))
  (bind _returnvalue (`KismetMathLibrary.MakeRotFromX` (`KismetMathLibrary.InverseTransformDirection` (`self.GetTransform`) (- (`self.TargetLocation`) (`SceneComponent.K2_GetComponentLocation` (`self.CannonMesh`))))))
  (`/Engine/EditorBlueprintResources/StandardMacros.IsValid` (`self.CurrentTarget`)
    (:`Is Valid`
      (`/Engine/EditorBlueprintResources/StandardMacros.Gate` true :!label _label
        (:`Exit`
          (`/Engine/EditorBlueprintResources/StandardMacros.IsValid` _currenttarget
            (:`Is Valid`
              (set `self.TargetLocation` (`self.K2_GetActorLocation` _currenttarget))
              (set `self.TargetAimRoatator` _returnvalue)
              (`SceneComponent.K2_SetRelativeRotation` (`self.PlatformMesh`) (`KismetMathLibrary.RInterpTo_Constant` (`SceneComponent.RelativeRotation` (`self.PlatformMesh`)) (`KismetMathLibrary.MakeRotator` 0.0 0.0 (.yaw _returnvalue)) (`GameplayStatics.GetWorldDeltaSeconds`) _turretaimingspeed) false false)
              (`SceneComponent.K2_SetRelativeRotation` (`self.CannonMesh`) (`KismetMathLibrary.MakeRotator` (.roll (`KismetMathLibrary.RInterpTo_Constant` (`SceneComponent.RelativeRotation` (`self.CannonMesh`)) (`KismetMathLibrary.MakeRotator` 0.0 (.pitch _returnvalue)) (`GameplayStatics.GetWorldDeltaSeconds`) _turretaimingspeed)) (`KismetMathLibrary.ClampAngle` (.pitch (`KismetMathLibrary.RInterpTo_Constant` (`SceneComponent.RelativeRotation` (`self.CannonMesh`)) (`KismetMathLibrary.MakeRotator` 0.0 (.pitch _returnvalue)) (`GameplayStatics.GetWorldDeltaSeconds`) _turretaimingspeed)) (`self.TurretMinAngle`) (`self.TurretMaxAngle`)) (.yaw (`KismetMathLibrary.RInterpTo_Constant` (`SceneComponent.RelativeRotation` (`self.CannonMesh`)) (`KismetMathLibrary.MakeRotator` 0.0 (.pitch _returnvalue)) (`GameplayStatics.GetWorldDeltaSeconds`) _turretaimingspeed))) false false)
              (if (== (`self.TargetAimRoatator`) (`KismetMathLibrary.MakeRotator` 0.0 (.pitch (`SceneComponent.RelativeRotation` (`self.CannonMesh`))) (.yaw (`SceneComponent.RelativeRotation` (`self.PlatformMesh`)))) :`ErrorTolerance` 1.0)
                (`|ExecutionSequence`
                  (:`then_0`
                    (set `self.ShootingPossible` true)
                    (`self.Shoot`))
                  (:`then_1`
                    (`KismetSystemLibrary.Delay` (`GameplayStatics.GetWorldDeltaSeconds`))
                    (`self.ContinueAiming`)))
                (else
                  (`KismetSystemLibrary.Delay` (`GameplayStatics.GetWorldDeltaSeconds`))
                  (`self.ContinueAiming`)
                  (set `self.ShootingPossible` false))))
            (:`Is Not Valid`
              (`self.CancelAim` :!label _label_2)
              (`self.BeginReset`))))))
    (:`Is Not Valid`
      (goto _label_2))))

(event `StartAiming`
  (`|ExecutionSequence`
    (:`then_0`
      (goto _label :!via `Open`))
    (:`then_1`
      (goto _label))))

(event `CancelAim`
  (goto _label :!via `Close`))

(event `ContinueReset`
  (bind _returnvalue (`KismetMathLibrary.RInterpTo_Constant` (`SceneComponent.RelativeRotation` (`self.CannonMesh`)) (struct) (`GameplayStatics.GetWorldDeltaSeconds`) 50.0))
  (bind _returnvalue_2 (`KismetMathLibrary.RInterpTo_Constant` (`SceneComponent.RelativeRotation` (`self.PlatformMesh`)) (struct) (`GameplayStatics.GetWorldDeltaSeconds`) 50.0))
  (`/Engine/EditorBlueprintResources/StandardMacros.Gate` true :!label _label_3
    (:`Exit`
      (`/Engine/EditorBlueprintResources/StandardMacros.IsValid` (`self.CurrentTarget`)
        (:`Is Valid`
          (`self.CancelReset` :!label _label_4))
        (:`Is Not Valid`
          (if (and (== _returnvalue_2 (struct)) (== _returnvalue (struct)))
            (goto _label_4)
            (else
              (`SceneComponent.K2_SetRelativeRotation` (`self.PlatformMesh`) _returnvalue_2 false false)
              (`SceneComponent.K2_SetRelativeRotation` (`self.CannonMesh`) _returnvalue false false)
              (`KismetSystemLibrary.Delay` (`GameplayStatics.GetWorldDeltaSeconds`))
              (`self.ContinueReset`))))))))

(event `BeginReset`
  (`|ExecutionSequence`
    (:`then_0`
      (goto _label_3 :!via `Open`))
    (:`then_1`
      (goto _label_3))))

(event `CancelReset`
  (goto _label_3 :!via `Close`))

(fn `UserConstructionScript`)