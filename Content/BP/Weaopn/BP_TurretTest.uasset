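; Test turret that tracks BP_TypeA actors inside its Sphere1 overlap, picking a random one as its target.
; A gated per-frame Delay loop turns the AnimBP's ToRotation toward the target with clamped pitch, calling Shoot once aligned.
; A second gated loop eases rotation back to zero when no target remains.
; Shoot is empty; the delayed twin-socket BP_Projectile spawn is disconnected and never runs.
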(event `Shoot`)

(event `self.ReceiveBeginPlay`
  (bind _assk_prop_turret_base_double_06_skeleton_anim_blueprint (cast `/Game/PolygonSciFiSpace/Meshes/Weapons/SK_Prop_Turret_Base_Double_06_Skeleton_AnimBlueprint` (`SkeletalMeshComponent.GetAnimInstance` (`self.SkeletalMesh`))))
  (set `self.AnimInstance` _assk_prop_turret_base_double_06_skeleton_anim_blueprint)
  (`self.FindTarget`))

(event `self.Sphere1.OnComponentBeginOverlap`
  (params (OverlappedComponent :type "PrimitiveComponent Object Reference") (OtherActor :type "Actor Object Reference") (OtherComp :type "PrimitiveComponent Object Reference") (OtherBodyIndex :type Integer) (bFromSweep :type Boolean) (SweepResult :type "HitResult Structure (by ref)"))
  (bind _asbp_type_a (cast `/Game/BP/Fighters/BP_TypeA` OtherActor))
  (`KismetArrayLibrary.Array_Add` (`self.Target Range`) _asbp_type_a)
  (`/Engine/EditorBlueprintResources/StandardMacros.IsValid` (`self.CurrentTarget`)
    (:`Is Not Valid`
      (`self.FindTarget`)
      (set `self.Shoot Possible` true))))

(event `self.Sphere1.OnComponentEndOverlap`
  (params (OverlappedComponent :type "PrimitiveComponent Object Reference") (OtherActor :type "Actor Object Reference") (OtherComp :type "PrimitiveComponent Object Reference") (OtherBodyIndex :type Integer))
  (bind _asbp_type_a (cast `/Game/BP/Fighters/BP_TypeA` OtherActor))
  (if (`KismetArrayLibrary.Array_Contains` (`self.Target Range`))
    (`KismetArrayLibrary.Array_RemoveItem` (`self.Target Range`))
    (if (== _asbp_type_a (`self.CurrentTarget`))
      (set `self.CurrentTarget` null)
      (`self.FindTarget`)
      (set `self.Shoot Possible` false))))

(event `FindTarget`
  (bind _target_range (`self.Target Range`))
  (if (`KismetArrayLibrary.Array_IsValidIndex` _target_range)
    (set `self.CurrentTarget` (`|GetArrayItem` _target_range (`KismetMathLibrary.RandomIntegerInRange` 0 (`KismetArrayLibrary.Array_LastIndex` _target_range))))
    (`self.StartAiming`)))

(event `ContinueAiming`
  (bind _currenttarget (`self.CurrentTarget`))
  (bind _returnvalue (`KismetMathLibrary.FindLookAtRotation` (`SceneComponent.GetSocketLocation` (`self.SkeletalMesh`) "Fire0") (`self.TargetLocation`)))
  (`/Engine/EditorBlueprintResources/StandardMacros.IsValid` (`self.CurrentTarget`)
    (:`Is Valid`
      (`/Engine/EditorBlueprintResources/StandardMacros.Gate` true :!label _label
        (:`Exit`
          (`/Engine/EditorBlueprintResources/StandardMacros.IsValid` _currenttarget
            (:`Is Valid`
              (set `self.TargetLocation` (`self.K2_GetActorLocation` _currenttarget))
              (set `/Game/PolygonSciFiSpace/Meshes/Weapons/SK_Prop_Turret_Base_Double_06_Skeleton_AnimBlueprint.FireLocation` (struct) (`self.AnimInstance`))
              (set `self.TargetAimRotator` _returnvalue)
              (set `/Game/PolygonSciFiSpace/Meshes/Weapons/SK_Prop_Turret_Base_Double_06_Skeleton_AnimBlueprint.ToRotation` (`KismetMathLibrary.RInterpTo_Constant` (`/Game/PolygonSciFiSpace/Meshes/Weapons/SK_Prop_Turret_Base_Double_06_Skeleton_AnimBlueprint.ToRotation` (`self.AnimInstance`)) (`KismetMathLibrary.MakeRotator` 0.0 (`KismetMathLibrary.ClampAngle` (.pitch (`KismetMathLibrary.MakeRotator` 0.0 (.pitch _returnvalue) (.yaw _returnvalue))) (`self.Turret Min Angle`) (`self.Turrent Max Angle`)) (.yaw (`KismetMathLibrary.MakeRotator` 0.0 (.pitch _returnvalue) (.yaw _returnvalue)))) (`GameplayStatics.GetWorldDeltaSeconds`) (`self.AimSpeed`)) (`self.AnimInstance`))
              (if (== (`self.TargetAimRotator`) (`KismetMathLibrary.MakeRotator` 0.0 (.pitch (`/Game/PolygonSciFiSpace/Meshes/Weapons/SK_Prop_Turret_Base_Double_06_Skeleton_AnimBlueprint.ToRotation` (`self.AnimInstance`))) (.yaw (`/Game/PolygonSciFiSpace/Meshes/Weapons/SK_Prop_Turret_Base_Double_06_Skeleton_AnimBlueprint.ToRotation` (`self.AnimInstance`)))) :`ErrorTolerance` 1.0)
                (`|ExecutionSequence`
                  (:`then_0`
                    (set `self.Shoot Possible` true)
                    (`self.Shoot`))
                  (:`then_1`
                    (`KismetSystemLibrary.Delay` (`GameplayStatics.GetWorldDeltaSeconds`))
                    (`self.ContinueAiming`)))
                (else
                  (`KismetSystemLibrary.Delay` (`GameplayStatics.GetWorldDeltaSeconds`))
                  (`self.ContinueAiming`)
                  (set `self.Shoot Possible` false))))
            (:`Is Not Valid`
              (`self.CancelAim` :!label _label_2)
              (`self.BeginReset`))))))
    (:`Is Not Valid`
      (goto _label_2))))

(event `StartAiming`
  (`|ExecutionSequence`
    (:`then_0`
      (goto _label :!via `Open`))
    (:`then_1`
      (goto _label))))

(event `CancelAim`
  (goto _label :!via `Close`))

(event `ContinueReset`
  (bind _returnvalue (`KismetMathLibrary.RInterpTo_Constant` (`/Game/PolygonSciFiSpace/Meshes/Weapons/SK_Prop_Turret_Base_Double_06_Skeleton_AnimBlueprint.ToRotation` (`self.AnimInstance`)) (struct) (`GameplayStatics.GetWorldDeltaSeconds`) 50.0))
  (`/Engine/EditorBlueprintResources/StandardMacros.Gate` true :!label _label_3
    (:`Exit`
      (`/Engine/EditorBlueprintResources/StandardMacros.IsValid` (`self.CurrentTarget`)
        (:`Is Valid`
          (`self.CancelReset` :!label _label_4))
        (:`Is Not Valid`
          (if (== _returnvalue (struct) :`ErrorTolerance` 0.0001)
            (goto _label_4)
            (else
              (set `/Game/PolygonSciFiSpace/Meshes/Weapons/SK_Prop_Turret_Base_Double_06_Skeleton_AnimBlueprint.ToRotation` _returnvalue (`self.AnimInstance`))
              (`KismetSystemLibrary.Delay` (`GameplayStatics.GetWorldDeltaSeconds`))
              (`self.ContinueReset`))))))))

(event `BeginReset`
  (`|ExecutionSequence`
    (:`then_0`
      (goto _label_3 :!via `Open`))
    (:`then_1`
      (goto _label_3))))

(event `CancelReset`
  (goto _label_3 :!via `Close`))

(fn `UserConstructionScript`)